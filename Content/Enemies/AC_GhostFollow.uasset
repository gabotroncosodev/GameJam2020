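; Actor component for a ghost enemy that steers its owning character toward either the player or the ProtectDog.
; BeginPlay caches the owner, the player character and a one-time snapshot of the dog's location, which it prints.
; Every Tick issues an AI move toward the player, then immediately another toward the player if GhostSeePlayer is true, otherwise to the saved dog location.
; GhostSeePlayer is only read here, never set.
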(event `self.ReceiveBeginPlay`
  (bind _ascharacter (cast `Character` (`self.GetOwner`)))
  (set `self.GetGhostFollower` _ascharacter) ; Obtiene fantasma
  (bind _asprincipal_character_bp (cast `/Game/PrincipalCharacter/PrincipalCharacterBP` (`GameplayStatics.GetPlayerCharacter` 0)))
  (set `self.GetCharacterFollow` _asprincipal_character_bp) ; Obtiene jugador
  (bind _returnvalue (`GameplayStatics.GetActorOfClass` "/Game/NPC/ProtectDog.ProtectDog_C"))
  (bind _output_get (set `self.DogPosition` (`Actor.K2_GetActorLocation` _returnvalue)))
  (`KismetSystemLibrary.PrintString` (`KismetStringLibrary.Conv_VectorToString` _output_get)))

(event `self.ReceiveTick`
  (params (DeltaSeconds :type "Float (single-precision)"))
  (`|AIMoveTo` (`self.GetGhostFollower`) (0.0 0.0 0.0) (`self.GetCharacterFollow`)
    (:`then`
      (if (`self.GhostSeePlayer`)
        (`|AIMoveTo` (`self.GetGhostFollower`) (0.0 0.0 0.0) (cast `/Game/PrincipalCharacter/PrincipalCharacterBP` (`GameplayStatics.GetPlayerCharacter` 0) :!pure true))
        (else
          (`|AIMoveTo` (`self.GetGhostFollower`) (`self.DogPosition`) null))))))